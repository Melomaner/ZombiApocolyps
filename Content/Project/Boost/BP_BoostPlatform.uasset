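; BP_BoostPlatform is a boost pickup platform that powers up a BP_Char overlapping its Sphere.
; On overlap it calls PowerUp on the character, disables the Sphere's collision, hides it and calls the TakeBoost dispatcher.
; An AddBoost event re-arms the pickup by showing the Sphere and restoring query-only collision.
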(event OnComponentBeginOverlap(Sphere)
  (params (OverlappedComponent :type Primitive%20Component%20Object%20Reference) (OtherActor :type Actor%20Object%20Reference) (OtherComp :type Primitive%20Component%20Object%20Reference) (OtherBodyIndex :type Integer) (bFromSweep :type Boolean) (SweepResult :type Hit%20Result%20Structure%20%28by%20ref%29))
  (bind _sphere (Variables|Default|GetSphere))
  (bind _asbp_char (Utilities|Casting|CastToBP_Char OtherActor))
  (Default|PowerUp _asbp_char)
  (Collision|SetCollisionEnabled _sphere "NoCollision")
  (Rendering|SetVisibility _sphere false false)
  (Default|CallTakeBoost))

(event Custom|AddBoost
  (Rendering|SetVisibility (Variables|Default|GetSphere) true false)
  (Collision|SetCollisionEnabled (Variables|Default|GetSphere) "QueryOnly"))

(fn ConstructionScript)