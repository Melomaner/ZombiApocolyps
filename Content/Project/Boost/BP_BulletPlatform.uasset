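; BP_BulletPlatform is a boost pickup that changes the player character's bullet color to Red, Green or Blue.
; SwitchBullet stores a color and reveals the matching component with query-only collision, without hiding the others.
; When BP_Char overlaps a component, it receives ChangeBullet with the stored color, and that component hides and disables its collision until switched on again.
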(event OnComponentBeginOverlap(Red)
  (params (OverlappedComponent :type Primitive%20Component%20Object%20Reference) (OtherActor :type Actor%20Object%20Reference) (OtherComp :type Primitive%20Component%20Object%20Reference) (OtherBodyIndex :type Integer) (bFromSweep :type Boolean) (SweepResult :type Hit%20Result%20Structure%20%28by%20ref%29))
  (bind _red (Variables|Default|GetRed))
  (bind _asbp_char (Utilities|Casting|CastToBP_Char OtherActor))
  (Default|ChangeBullet _asbp_char (Variables|Default|GetColor))
  (Collision|SetCollisionEnabled _red "NoCollision")
  (Rendering|SetVisibility _red false false))

(event OnComponentBeginOverlap(Blue)
  (params (OverlappedComponent :type Primitive%20Component%20Object%20Reference) (OtherActor :type Actor%20Object%20Reference) (OtherComp :type Primitive%20Component%20Object%20Reference) (OtherBodyIndex :type Integer) (bFromSweep :type Boolean) (SweepResult :type Hit%20Result%20Structure%20%28by%20ref%29))
  (bind _blue (Variables|Default|GetBlue))
  (bind _asbp_char (Utilities|Casting|CastToBP_Char OtherActor))
  (Default|ChangeBullet _asbp_char (Variables|Default|GetColor))
  (Collision|SetCollisionEnabled _blue "NoCollision")
  (Rendering|SetVisibility _blue false false))

(event OnComponentBeginOverlap(Green)
  (params (OverlappedComponent :type Primitive%20Component%20Object%20Reference) (OtherActor :type Actor%20Object%20Reference) (OtherComp :type Primitive%20Component%20Object%20Reference) (OtherBodyIndex :type Integer) (bFromSweep :type Boolean) (SweepResult :type Hit%20Result%20Structure%20%28by%20ref%29))
  (bind _green (Variables|Default|GetGreen))
  (bind _asbp_char (Utilities|Casting|CastToBP_Char OtherActor))
  (Default|ChangeBullet _asbp_char (Variables|Default|GetColor))
  (Collision|SetCollisionEnabled _green "NoCollision")
  (Rendering|SetVisibility _green false false))

(event Custom|SwitchBullet
  (params (Color :type Name))
  (bind _output_get (Variables|Default|SetColor Color))
  (switch name _output_get
    (:Red
      (Rendering|SetVisibility (Variables|Default|GetRed) true false)
      (Collision|SetCollisionEnabled (Variables|Default|GetRed) "QueryOnly"))
    (:Green
      (Rendering|SetVisibility (Variables|Default|GetGreen) true false)
      (Collision|SetCollisionEnabled (Variables|Default|GetGreen) "QueryOnly"))
    (:Blue
      (Rendering|SetVisibility (Variables|Default|GetBlue) true false)
      (Collision|SetCollisionEnabled (Variables|Default|GetBlue) "QueryOnly"))))

(fn ConstructionScript)