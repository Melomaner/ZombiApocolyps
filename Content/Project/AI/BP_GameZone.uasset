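; BP_GameZone is a zone actor that spawns one colored spawner and one bullet platform on BeginPlay.
; Both spawn at random points in the Plane's bounds facing Center, retrying overlapping spots against a shared LimitBad failure cap.
; The spawner gets a random red, green or blue sphere and increments that color's tally.
; The platform's bullet color is then rolled against those tallies, with blue as the fallback.
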(event EventBeginPlay
  (bind (_successfull _spawner) (CallFunction|SpawnNewSpawner))
  (if _successfull
    (CallFunction|SetSetingsSpawner _spawner)
    (bind (_successfull_2 _bullet) (CallFunction|SpawnNewBullet))
    (if _successfull_2
      (CallFunction|SetSetingsBulletifAddSpawner _bullet))))

(fn ConstructionScript)

(fn SpawnNewSpawner
  (bind _plane (Variables|Default|GetPlane))
  (bind (_origin _boxextent) (Collision|GetComponentBounds _plane))
  ;[1 1 1] Take a random point at the location
  (bind _output_get (LocalVariables|SetPointSpawn (Math|Random|RandomPointinBoundingBox _origin _boxextent) :!label _label))
  ;[1 1 1] Check if space is free
  (bind _returnvalue (Collision|BoxOverlapComponents _output_get "700.000000,500.000000,1000.000000" (LocalVariables|GetCheckObjs) 0 0 :!class /Script/Engine.KismetSystemLibrary))
  (if _returnvalue
    ;[1 0.1863 0.1664] Debugging on the fullness of the location
    (bind _result (Math|Integer|IncrementInt (LocalVariables|GetLimitBad))
      (:%20%20
        (if (>= _result 10)
          (return false 0)
          (else
            (goto _label)))))
    (else
      ;[1 1 1] If the space is free, then spawn the spawner
      (bind _returnvalue_2 (Game|SpawnActorfromClass "/Game/Project/AI/BP_Spawner.BP_Spawner_C" (Math|Transform|MakeTransform (LocalVariables|GetPointSpawn) (Math|Rotator|FindLookatRotation (LocalVariables|GetPointSpawn) (Transformation|GetActorLocation (Variables|Default|GetCenter))) "1,1,1") "Undefined" 0 0))
      (Utilities|IsValid _returnvalue_2
        (:Is%20Valid
          (return true _returnvalue_2))
        (:Is%20Not%20Valid
          (return false 0))))))

(fn SetSetingsSpawner
  (params (InputPin :type BP%20Spawner%20Object%20Reference))
  (switch int (Math|Random|RandomIntegerinRange 1 3)
    (:1
      (Default|SetRedSphere InputPin)
      (Math|Integer|IncrementInt (Variables|Default|GetSumRedSpawner)))
    (:2
      (Default|SetGreenSphere InputPin)
      (Math|Integer|IncrementInt (Variables|Default|GetSumGreenSpawner)))
    (:3
      (Default|SetBlueSphere InputPin)
      (Math|Integer|IncrementInt (Variables|Default|GetSumBlueSpawner)))))

(fn SpawnNewBullet
  (bind _plane (Variables|Default|GetPlane))
  (bind (_origin _boxextent) (Collision|GetComponentBounds _plane))
  ;[1 1 1] Take a random point at the location
  (bind _output_get (LocalVariables|SetPointSpawn (Math|Random|RandomPointinBoundingBox _origin _boxextent) :!label _label))
  ;[1 1 1] Check if space is free
  (bind _returnvalue (Collision|BoxOverlapComponents _output_get "700.000000,500.000000,1000.000000" (LocalVariables|GetCheckObjs) 0 0 :!class /Script/Engine.KismetSystemLibrary))
  (if _returnvalue
    ;[1 0.1863 0.1664] Debugging on the fullness of the location
    (bind _result (Math|Integer|IncrementInt (LocalVariables|GetLimitBad))
      (:%20%20
        (if (>= _result 10)
          (return false 0)
          (else
            (goto _label)))))
    (else
      ;[1 1 1] If the space is free, then spawn the spawner
      (bind _returnvalue_2 (Game|SpawnActorfromClass "/Game/Project/Boost/BP_BulletPlatform.BP_BulletPlatform_C" (Math|Transform|MakeTransform (LocalVariables|GetPointSpawn) (Math|Rotator|FindLookatRotation (LocalVariables|GetPointSpawn) (Transformation|GetActorLocation (Variables|Default|GetCenter))) "1,1,1") "Undefined" 0 0))
      (Utilities|IsValid _returnvalue_2
        (:Is%20Valid
          (return true _returnvalue_2))
        (:Is%20Not%20Valid
          (return false 0))))))

(fn SetSetingsBulletifAddSpawner
  (params (InputPin :type BP%20Bullet%20Platform%20Object%20Reference))
  (bind _sumgreenspawner (Variables|Default|GetSumGreenSpawner))
  (bind _sumredspawner (Variables|Default|GetSumRedSpawner))
  (LocalVariables|SetBulletPlatphorm InputPin)
  (bind _output_get (LocalVariables|SetRandomRange (Math|Random|RandomFloatinRange 0.0 1.0)))
  (if (and (<= _output_get (/ (Math|Conversions|ToFloat(Integer) _sumredspawner) (Math|Conversions|ToFloat(Integer) (+ _sumredspawner (Variables|Default|GetSumGreenSpawner) (Variables|Default|GetSumBlueSpawner))))) (!= _sumredspawner 0))
    (Default|SwitchBullet (LocalVariables|GetBulletPlatphorm) "Red")
    (elif (and (<= (LocalVariables|GetRandomRange) (/ (Math|Conversions|ToFloat(Integer) _sumgreenspawner) (Math|Conversions|ToFloat(Integer) (+ (Variables|Default|GetSumRedSpawner) _sumgreenspawner (Variables|Default|GetSumBlueSpawner))))) (!= _sumgreenspawner 0))
      (Default|SwitchBullet (LocalVariables|GetBulletPlatphorm) "Green")
      (else
        (Default|SwitchBullet (LocalVariables|GetBulletPlatphorm) "Blue")))))