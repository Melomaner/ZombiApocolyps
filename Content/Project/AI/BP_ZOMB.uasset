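; BP_ZOMB is a zombie character that takes damage, dies as a ragdoll and then despawns.
; Point damage reduces HP, with doubled damage for hits on the Head bone, and triggers Die once at zero.
; Die spawns a gore explosion on the mesh, disables capsule collision, simulates physics from the Hips down, then destroys the actor after a short delay.
; SetWalkSpeed scales the movement speed by the WalkSpeed variable.
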(event Custom|Die
  (bind _returnvalue (Utilities|Name|MakeLiteralName "Hips"))
  (bind _mesh (Variables|Character|GetMesh))
  (Variables|Default|SetDead true)
  (Effects|SpawnEmitterAttached "/Game/Project/Particles/P_ExplosionMeet.P_ExplosionMeet" (Variables|Character|GetMesh) "None")
  (Collision|SetCollisionEnabled (Variables|Collision|GetCapsuleComponent) "NoCollision")
  (Collision|SetCollisionEnabled _mesh "QueryAndPhysics")
  (Variables|/Script/Engine.SkeletalMeshComponent|SetbPauseAnims _mesh true)
  (Components|Activation|Activate _mesh false)
  (Class|SkeletalMeshComponent|SetAllBodiesBelowSimulatePhysics _mesh _returnvalue true true)
  (Class|SkeletalMeshComponent|SetAllBodiesBelowPhysicsBlendWeight _mesh _returnvalue 1.0 false true)
  (Utilities|FlowControl|Delay 2.0)
  (Actor|DestroyActor))

(event EventBeginPlay)

(event Collision|EventActorBeginOverlap
  (params (OtherActor :type Actor%20Object%20Reference)))

(event EventTick
  (params (DeltaSeconds :type Float%20%28single-precision%29)))

(event Game|Damage|EventPointDamage
  (params (Damage :type Float%20%28single-precision%29) (DamageType :type Damage%20Type%20Object%20Reference) (HitLocation :type Vector :default "0, 0, 0") (HitNormal :type Vector :default "0, 0, 0") (HitComponent :type Primitive%20Component%20Object%20Reference) (BoneName :type Name :default "None") (ShotFromDirection :type Vector :default "0, 0, 0") (InstigatedBy :type Controller%20Object%20Reference) (DamageCauser :type Actor%20Object%20Reference) (HitInfo :type Hit%20Result%20Structure%20%28by%20ref%29))
  (bind _output_get (Variables|Default|SetHP (- (Variables|Default|GetHP) (select (Utilities|Name|Equal(Name) BoneName "Head") (* Damage 2.0) Damage))))
  (if (and (<= _output_get 0.0) (not (Variables|Default|GetDead)))
    (CallFunction|Die)))

(fn ConstructionScript)

(fn SetWalkSpeed
  (params (Speed :type Float%20%28single-precision%29))
  (Variables|/Script/Engine.CharacterMovementComponent|SetMaxWalkSpeed (Variables|Character|GetCharacterMovement) (* Speed (Variables|Default|GetWalkSpeed))))