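; BP_Spawner is a destructible spawner that produces BP_ZOMB actors at random points within the SpawnPawn bounds.
; Tick drives a countdown macro that triggers spawns, pausing at the live zombie cap and resuming as deaths lower the count.
; A color-matching macro filters bullet damage types, but only RedSphere hits reduce Health.
; At zero Health it stops spawning, disables collision, toggles RedSphere visibility and starts a one-second timer.
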(event Custom|Destroy
  (Actor|DestroyActor))

(event Custom|StartSpawn
  (Variables|Default|SetSpawnWork true))

(event EventTick
  (params (DeltaSeconds :type Float%20%28single-precision%29))
  (if (Variables|Default|GetSpawnWork)
    (Utilities|TimerSpawn DeltaSeconds)
    (CallFunction|SpawnZombi 0.0)))

(event Game|Damage|EventPointDamage
  (params (Damage :type Float%20%28single-precision%29) (DamageType :type Damage%20Type%20Object%20Reference) (HitLocation :type Vector :default "0, 0, 0") (HitNormal :type Vector :default "0, 0, 0") (HitComponent :type Primitive%20Component%20Object%20Reference) (BoneName :type Name :default "None") (ShotFromDirection :type Vector :default "0, 0, 0") (InstigatedBy :type Controller%20Object%20Reference) (DamageCauser :type Actor%20Object%20Reference) (HitInfo :type Hit%20Result%20Structure%20%28by%20ref%29))
  (bind _redsphere (Variables|Default|GetRedSphere))
  (Utilities|CheckBullet DamageType
    (:OutputPin
      (if (== HitComponent _redsphere)
        (Audio|SpawnSoundatLocation "/Game/Project/Sound/Obj/Glass/Cue_Crack.Cue_Crack" (Variables|/Script/Engine.SceneComponent|GetRelativeLocation _redsphere) "0, 0, 0" 1.0 1.0 0.0 0 0)
        (bind _output_get (Variables|Default|SetHealth (- (Variables|Default|GetHealth) Damage)))
        (if (<= _output_get 0.0)
          (CallFunction|DestroySpawner))))))

(fn ConstructionScript)

(fn SpawnZombi
  (params (EventTick :type Float%20%28single-precision%29))
  (bind _spawnpawn (Variables|Default|GetSpawnPawn))
  (bind (_origin _boxextent) (Collision|GetComponentBounds _spawnpawn))
  (bind _returnvalue (Game|SpawnActorfromClass "/Game/Project/AI/BP_ZOMB.BP_ZOMB_C" (Math|Transform|MakeTransform (Math|Random|RandomPointinBoundingBox _origin _boxextent) "0, 0, 0" "1,1,1") "Undefined" 0 0))
  (Utilities|IsValid _returnvalue
    (:Is%20Valid
      (bind _output_get (Variables|Default|SetNewZombi _returnvalue))
      (Game|BindEventtoOnDestroyed _output_get (EventDispatchers|CreateEvent :!event ZombiDead))
      (bind _result (Math|Integer|IncrementInt (Variables|Default|GetCountLiveZombi))
        (:%20%20
          (if (>= _result (Variables|Default|GetMaxCountLiveZombi))
            (Variables|Default|SetSpawnWork false)
            (return)
            (else
              (return))))))
    (:Is%20Not%20Valid
      (return))))

(fn ZombiDead
  (params (DeadZombi :type Actor%20Object%20Reference))
  (Default|CallKillsZombi)
  (bind _result (Math|Integer|DecrementInt (Variables|Default|GetCountLiveZombi))
    (:%20%20
      (if (not (>= _result (Variables|Default|GetMaxCountLiveZombi)))
        (Variables|Default|SetSpawnWork true)))))

(fn BPSpawnerAutoGenFunc
  (params (DestroyedActor :type Actor%20Object%20Reference)))

(fn DestroySpawner
  (Variables|Default|SetSpawnWork false)
  (Collision|SetActorEnableCollision false)
  (Rendering|ToggleVisibility (Variables|Default|GetRedSphere) false)
  (Utilities|Time|SetTimerbyEvent (EventDispatchers|CreateEvent :!event Custom|Destroy) 1.0))

(fn SetRedSphere
  (Rendering|SetVisibility (Variables|Default|GetRedSphere) true false)
  (Variables|Default|SetColor "Red"))

(fn SetGreenSphere
  (Rendering|SetVisibility (Variables|Default|GetGreenSphere) true false)
  (Variables|Default|SetColor "Green"))

(fn SetBlueSphere
  (Rendering|SetVisibility (Variables|Default|GetBlueSphere) true true)
  (Variables|Default|SetColor "Blue"))